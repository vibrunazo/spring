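; Hit spark actor that shows a point light which fades out after it spawns.
; On BeginPlay it sets the light to its starting intensity and starts a looping timer.
; Each timer tick subtracts a fixed step from the stored intensity, clamps it at zero and applies it to the light.
; The timer is never cleared and the actor is not destroyed in this Blueprint's graphs.
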(event Custom|reduce%20light
  (Utilities|FlowControl|Sequence
    (:then_0
      (|setcurrentintensity))
    (:then_1
      (|updatelightintensity))))

(event EventBeginPlay
  (Utilities|FlowControl|Sequence
    (:then_0
      (|Setinitiallightintensity))
    (:then_1
      (|Settimertoreducelight (delegate Custom|reduce%20light)))))

(event EventActorBeginOverlap
  (params (OtherActor :type Actor%20Object%20Reference)))

(event EventTick
  (params (DeltaSeconds :type Float%20%28single-precision%29)))

(fn ConstructionScript)