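; Area actor that tracks a paused Manny and calls UnPause on him once no living Enemy_1 remains nearby.
; Box overlap stores the Manny reference and sets a paused flag, but does not itself pause him or run a check.
; Enemies entering or leaving the Sphere trigger recounts of live, capsule-overlapping enemies while flagged; the flag is never cleared.
; The construction script sizes the Sphere from RangeForEnemies, converting metres to centimetres.
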(event OnComponentBeginOverlap(Sphere)
  (params (OtherActor :type Actor%20Object%20Reference) (OtherComp :type Primitive%20Component%20Object%20Reference) (OtherBodyIndex :type Integer) (bFromSweep :type Boolean) (SweepResult :type Hit%20Result%20Structure%20%28by%20ref%29))
  (Utilities|Casting|CastToEnemy_1 OtherActor)
  (CallFunction|CheckforEnemies))

(event OnComponentEndOverlap(Sphere)
  (params (OtherActor :type Actor%20Object%20Reference) (OtherComp :type Primitive%20Component%20Object%20Reference) (OtherBodyIndex :type Integer))
  (Utilities|Casting|CastToEnemy_1 OtherActor)
  (CallFunction|CheckforEnemies))

(event OnComponentBeginOverlap(Box)
  (params (OtherActor :type Actor%20Object%20Reference) (OtherComp :type Primitive%20Component%20Object%20Reference) (OtherBodyIndex :type Integer) (bFromSweep :type Boolean) (SweepResult :type Hit%20Result%20Structure%20%28by%20ref%29))
  (bind _asmanny (Utilities|Casting|CastToManny OtherActor))
  (Variables|Default|SetManny%20reference _asmanny)
  (Variables|Default|SetIpaused true)
  (Development|PrintString "paused"))

(event Custom|Check%20for%20enemies
  (bind _manny_reference (Variables|Default|GetManny%20reference))
  (if (Variables|Default|GetIpaused)
    (Variables|Default|Setcount%20live%20enemies 0)
    (for _array_element (Collision|GetOverlappingActors (Variables|Default|GetSphere) "/Game/Blueprints/Actors/Characters/Enemy_1.Enemy_1_C" :!class /Script/Engine.PrimitiveComponent)
      (bind _asenemy_1 (Utilities|Casting|CastToEnemy_1 _array_element))
      (if (Variables|/Game/Blueprints/Actors/Characters/BaseChar.BaseChar_C|Getisalive _asenemy_1)
        (if (Class|PrimitiveComponent|IsOverlappingComponent (Variables|Default|GetSphere) (Variables|/Script/Engine.Character|GetCapsuleComponent _asenemy_1))
          (Math|Integer|IncrementInt (Variables|Default|Getcount%20live%20enemies)))))
    (if (== (Variables|Default|Getcount%20live%20enemies) 0)
      (Utilities|IsValid _manny_reference
        (:Is%20Valid
          (Default|UnPause _manny_reference))))))

(event EventBeginPlay
  (CallFunction|CheckforEnemies))

(event EventActorBeginOverlap
  (params (OtherActor :type Actor%20Object%20Reference)))

(event EventTick
  (params (DeltaSeconds :type Float%20%28single-precision%29)))

(fn ConstructionScript
  (|CallParentFunction)
  (Components|Sphere|SetSphereRadius (Variables|Default|GetSphere) (* (Variables|Trigger|GetRange%20for%20enemies) 1e+02) true))