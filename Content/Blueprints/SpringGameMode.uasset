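; SpringGameMode is a game mode Blueprint that owns the on-screen HUD and relays health and O2 values to it.
; A macro lazily creates the SpringHUD widget, adds it to the viewport and caches the reference.
; BeginPlay and both setter events run that macro, so the SetO2onUI and SetHealthonUI events create the HUD if it is missing before updating it.
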(event Custom|Set%20Health%20on%20UI
  (params (health :type Integer))
  (Utilities|CreateHUDifNeeded
    (:out
      (Default|SetHealth (Variables|Default|GetHUD%20reference) health))))

(event Custom|Set%20O2%20on%20UI
  (params (O2 :type Integer))
  (Utilities|CreateHUDifNeeded
    (:out
      (Default|SetO2 (Variables|Default|GetHUD%20reference) O2))))

(event EventBeginPlay
  (Utilities|CreateHUDifNeeded))

(event EventTick
  (params (DeltaSeconds :type Float%20%28single-precision%29)))

(fn ConstructionScript)